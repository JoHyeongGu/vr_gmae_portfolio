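; BP_GrabSpawner is an actor that adds GrabComponents to grabbable actors at runtime.
; On BeginPlay it scans every actor in the level and adds a GrabComponent to any with a SceneComponent tagged "GrabComponent".
; Separate events add a component to a given actor or destroy all GrabComponents on it.
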(event `self.ReceiveBeginPlay`
  (`self.AttachGrabComponentInAllGrabActors`))

(event `self.AttachGrabComponent`
  (params (TargetActor :type "Actor Object Reference"))
  (`AddComponent|NODE_AddGrabComponent-0` :`self` TargetActor))

(event `self.AttachGrabComponentInAllGrabActors`
  (bind _outactors (`GameplayStatics.GetAllActorsOfClass` "/Script/Engine.Actor"))
  (for _array_element _outactors
    (if (`KismetArrayLibrary.Array_IsNotEmpty` (`self.GetComponentsByTag` _array_element "/Script/Engine.SceneComponent" "GrabComponent"))
      (`|AddComponentByClass` :`self` _array_element :`Class` "/Game/VRTemplate/Blueprints/GrabComponent.GrabComponent_C"))))

(event `self.DeleteGrabComponent`
  (params (TargetActor :type "Actor Object Reference"))
  (for _array_element (`self.K2_GetComponentsByClass` TargetActor "/Game/VRTemplate/Blueprints/GrabComponent.GrabComponent_C")
    (`ActorComponent.K2_DestroyComponent` _array_element)))

(fn `UserConstructionScript`)